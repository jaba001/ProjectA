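; Test projectile actor that moves itself along world +Y by a fixed step every Tick, without sweep or delta-time scaling.
; After each move, a Delay in Tick gates activation of the NSMagmaShotOwnerCastSpell effect.
; Box overlap calls RequestImpact, and debug strings print on spawn, overlap and destruction.
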(event OnComponentBeginOverlap(Box)
  (params (OverlappedComponent :type Primitive%20Component%20Object%20Reference) (OtherActor :type Actor%20Object%20Reference) (OtherComp :type Primitive%20Component%20Object%20Reference) (OtherBodyIndex :type Integer) (bFromSweep :type Boolean) (SweepResult :type Hit%20Result%20Structure%20%28by%20ref%29))
  (Development|PrintString "overlap")
  (Class|SkillActorBase|RequestImpact))

(event EventBeginPlay
  (Development|PrintString "ActorSpawned"))

(event EventTick
  (params (DeltaSeconds :type Float%20%28single-precision%29))
  (Transformation|SetActorLocation (+ (Transformation|GetActorLocation) "0.000000,3.000000,0.000000") false false)
  (Utilities|FlowControl|Delay 1.4)
  (Components|Activation|Activate (Variables|Default|GetNS_Magma_Shot_Owner_Cast_Spell) true))

(event EventDestroyed
  (Development|PrintString "ActorEnd"))

(fn ConstructionScript)